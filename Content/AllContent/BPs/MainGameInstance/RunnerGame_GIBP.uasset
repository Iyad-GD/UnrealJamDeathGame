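; Game instance for the runner game that keeps a running points total and restores saved audio volumes at startup.
; On Init it sets the master sound mix, then loads the MusicVolume save slot, or creates and saves a new audio settings object if none is usable.
; The saved music and SFX volumes are applied as sound class overrides on that mix.
; AddPoints and GetPoints update and read the score.
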(event EventInit
  ;[0.15 0.15 0.15 0.5] Audio Permanence (DO NOT TOUCH)
  (Class|GameplayStatics|SetBaseSoundMix "/Game/AllContent/BPs/Audio/SoundMixer_Master.SoundMixer_Master")
  (bind _returnvalue (SaveGame|DoesSaveGameExist "MusicVolume"))
  (if _returnvalue
    (bind _returnvalue_2 (SaveGame|LoadGamefromSlot "MusicVolume"))
    (bind _assave_game_audio_settings_bp (Utilities|Casting|CastToSaveGameAudioSettings_BP _returnvalue_2)
      (:then
        (Variables|Default|SetVolumeSaver _assave_game_audio_settings_bp)
        (CallFunction|ApplyAudiofromSave))
      (:CastFailed
        (bind _returnvalue_3 (SaveGame|CreateSaveGameObject "/Game/AllContent/BPs/Audio/SaveGameAudioSettings_BP.SaveGameAudioSettings_BP_C" :!label _label))
        (bind _output_get (Variables|Default|SetVolumeSaver _returnvalue_3))
        (CallFunction|ApplyAudiofromSave)
        (SaveGame|SaveGametoSlot _output_get "MusicVolume")))
    (else
      (goto _label))))

(fn AddPoints
  (params (Amount :type Integer))
  (Variables|Default|SetPoints (+ (Variables|Default|GetPoints) Amount)))

(fn GetPoints
  (return (Variables|Default|GetPoints)))

(fn ApplyAudiofromSave
  (bind _volumesaver (Variables|Default|GetVolumeSaver)
    (:then
      (Audio|SetSoundMixClassOverride "/Game/AllContent/BPs/Audio/SoundMixer_Master.SoundMixer_Master" "/Game/AllContent/BPs/Audio/MainBGM/SC_Master.SC_Master" (Variables|/Game/AllContent/BPs/Audio/SaveGameAudioSettings_BP.SaveGameAudioSettings_BP_C|GetBGM_Sound _volumesaver) 1.0 0.0 true)
      (Audio|SetSoundMixClassOverride "/Game/AllContent/BPs/Audio/SoundMixer_Master.SoundMixer_Master" "/Game/AllContent/BPs/Audio/MainBGM/SC_SFX_Master.SC_SFX_Master" (Variables|/Game/AllContent/BPs/Audio/SaveGameAudioSettings_BP.SaveGameAudioSettings_BP_C|GetSFX_Sound _volumesaver) 1.0 0.0 true))
    (:else)))