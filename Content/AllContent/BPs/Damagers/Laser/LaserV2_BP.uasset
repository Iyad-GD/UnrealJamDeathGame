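; Laser hazard Blueprint that deals massive damage and plays an electrocution sound when the first-person character overlaps its box.
; Tick, throttled by a short Delay, line-traces along the arrow on the Camera channel and scales the laser's length to the hit point or full range.
; The construction script adds InterpToMovement control points at the origin and a relative Location, defining the laser's movement path.
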(event OnComponentBeginOverlap(Box)
  (params (OverlappedComponent :type Primitive%20Component%20Object%20Reference) (OtherActor :type Actor%20Object%20Reference) (OtherComp :type Primitive%20Component%20Object%20Reference) (OtherBodyIndex :type Integer) (bFromSweep :type Boolean) (SweepResult :type Hit%20Result%20Structure%20%28by%20ref%29))
  (bind _asbp_first_person_character (Utilities|Casting|CastToBP_FirstPersonCharacter OtherActor))
  (Audio|PlaySound2D "/Game/AllContent/BPs/Audio/SFX/electrocution.electrocution" 1.0 1.0 0.0 0 0)
  (Game|Damage|ApplyDamage _asbp_first_person_character 1e+03 0 0))

(event EventTick
  (params (DeltaSeconds :type Float%20%28single-precision%29))
  (bind _arrow (Variables|Default|GetArrow))
  (bind _returnvalue (Transformation|GetWorldLocation _arrow))
  ;[0.15 0.15 0.15 0.5] Laser Logic
  (Utilities|FlowControl|Delay 0.2)
  (bind (_outhit _returnvalue_2) (Collision|LineTraceByChannel _returnvalue (+ _returnvalue (* (Math|Vector|GetForwardVector _arrow) (Variables|HowLong?|GetLength))) "TraceTypeQuery2" false 0 "None"))
  (Transformation|SetRelativeScale3D (Variables|Default|GetLaser) (Math|Vector|MakeVector (/ (Math|Vector|VectorLength (- (select _returnvalue_2 (.Location (Collision|BreakHitResult _outhit)) (.TraceEnd (Collision|BreakHitResult _outhit))) (.TraceStart (Collision|BreakHitResult _outhit)))) 2e+02) 0.2 0.2)))

(fn ConstructionScript
  (Class|InterptoMovementComponent|AddControlPointPosition (Variables|Default|GetInterpToMovement) "0, 0, 0" true)
  (Class|InterptoMovementComponent|AddControlPointPosition (Variables|Default|GetInterpToMovement) (Variables|HowLong?|GetLocation) true))