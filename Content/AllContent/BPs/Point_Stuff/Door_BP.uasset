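; Key-locked double door that opens when a first-person character holding a key overlaps it.
; The overlap clears the character's HaveKey flag, then a DoOnce gate plays a 2D sound and the DoorOpen timeline, which swings both door leaves 90 degrees in opposite directions.
; The key is cleared before the gate, so later overlaps still consume a key without replaying the opening.
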(event EventBeginPlay)

(event EventTick
  (params (DeltaSeconds :type Float%20%28single-precision%29)))

(event Collision|EventActorBeginOverlap
  (params (OtherActor :type Actor%20Object%20Reference))
  (bind _asbp_first_person_character (Utilities|Casting|CastToBP_FirstPersonCharacter OtherActor))
  (if (Variables|/Game/AllContent/BPs/MainChar/BP_FirstPersonCharacter.BP_FirstPersonCharacter_C|GetHaveKey? _asbp_first_person_character)
    (Variables|/Game/AllContent/BPs/MainChar/BP_FirstPersonCharacter.BP_FirstPersonCharacter_C|SetHaveKey? _asbp_first_person_character false)
    (Utilities|FlowControl|DoOnce false
      (:Completed
        (Audio|PlaySound2D "/Game/AllContent/BPs/Audio/SFX/opening-door-450444.opening-door-450444" 0.5 1.0 0.2 0 0)
        (bind _dooropening (Timeline|DoorOpen Play)
          (:Update
            (Transformation|SetRelativeRotation (Variables|Default|GetLeftDoor) (Math|Rotator|Lerp(Rotator) "0, 0, 0" "0.000000,-90.000000,0.000000" _dooropening) false false)
            (Transformation|SetRelativeRotation (Variables|Default|GetRightDoor) (Math|Rotator|Lerp(Rotator) "0.000000,180.000000,0.000000" "0.000000,270.000000,0.000000" _dooropening) false false)))))))

(fn ConstructionScript)